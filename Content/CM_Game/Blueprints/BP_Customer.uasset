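; BP_Customer is a bar customer that gets a drink glass and scores how the player handles it.
; On BeginPlay it spawns a BP_Glass at its arrow using the first recipe from BP_Globals.
; A tagged glass overlapping DrinkSpot triggers DrinkComplete.
; Reaction maps intensity levels to score changes, sounds or debug prints, with a wrong-hand touch destroying customer and glass.
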(event `self.ReceiveBeginPlay`
  (bind _returnvalue (`GameplayStatics.GetActorOfClass` "/Game/CM_Game/Blueprints/BP_Globals.BP_Globals_C"))
  (bind _recipes (`/Game/CM_Game/Blueprints/BP_Globals.recipes` _returnvalue))
  (if (> (`KismetArrayLibrary.Array_Length` _recipes) 0)
    (`self.SpawnCup` (`|GetArrayItem` _recipes))))

(event `self.DrinkSpot.OnComponentBeginOverlap`
  (params (OverlappedComponent :type "PrimitiveComponent Object Reference") (OtherActor :type "Actor Object Reference") (OtherComp :type "PrimitiveComponent Object Reference") (OtherBodyIndex :type Integer) (bFromSweep :type Boolean) (SweepResult :type "HitResult Structure (by ref)"))
  (if (`self.ActorHasTag` "Glass")
    (bind _asbp_glass (cast `/Game/CM_Game/Blueprints/BP_Glass` OtherActor))
    (`/Game/CM_Game/Blueprints/BP_Glass.DrinkComplete` _asbp_glass)))

(fn `DestroyCustomer`
  (`self.K2_DestroyActor` (`self.myGlass`))
  (`self.K2_DestroyActor`))

(fn `Reaction`
  (params (reactionIntensity :type Integer))
  (bind _returnvalue (`GameplayStatics.GetActorOfClass` "/Game/CM_Game/Blueprints/BP_Globals.BP_Globals_C"))
  ;[1 1 1] Player Mixes Drink Correctly
  (if (== reactionIntensity 4)
    (bind _score (`/Game/CM_Game/Blueprints/BP_Globals.score` _returnvalue))
    (bind _output_get (set `/Game/CM_Game/Blueprints/BP_Globals.score` (+ _score 5) _returnvalue))
    (`KismetSystemLibrary.PrintString` (`KismetStringLibrary.Conv_IntToString` _output_get))
    (else
      ;[1 1 1] Player messes up Drink
      (if (== reactionIntensity 3)
        (set `/Game/CM_Game/Blueprints/BP_Globals.score` (+ _score 1) _returnvalue)
        (`KismetSystemLibrary.PrintString` (`KismetStringLibrary.Conv_IntToString` 0))
        (else
          ;[1 1 1] Player uses wrong Hand to touch glass
          (if (== reactionIntensity 2)
            (set `/Game/CM_Game/Blueprints/BP_Globals.score` (+ _score -10) _returnvalue)
            (`self.DestroyCustomer`)
            (`KismetSystemLibrary.PrintString` "KABOOOOOMMM!!!")
            (`GameplayStatics.PlaySoundAtLocation` "/Game/StarterContent/Audio/Explosion01.Explosion01" (0.0 0.0 0.0) (struct) 1.0 1.0 0.0 null null null)
            (else
              ;[1 1 1] ELSE Uses Correct Hand to Touch Glass
              (`GameplayStatics.PlaySoundAtLocation` "/Engine/VREditor/Sounds/UI/Camera_Shutter.Camera_Shutter" (0.0 0.0 0.0) (struct) 1.0 1.0 0.0 null null null))))))))

(fn `SpawnCup`
  (params (recipe :type "/Game/CM_Game/Blueprints/BP_Recipe Object Reference"))
  (bind _returnvalue (`|SpawnActorFromClass` "/Game/CM_Game/Blueprints/BP_Glass.BP_Glass_C" (`SceneComponent.K2_GetComponentToWorld` (`self.Arrow1`)) "Undefined" "OverrideRootScale" null 0.0 recipe self))
  (set `self.myGlass` _returnvalue))

(fn `UserConstructionScript`)