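; Bottle Blueprint that tracks its fill level and triggers a customer's reaction when it is held.
; BeingHeld compares the incoming hand type with the type of the bottle's instigator customer, calling one reaction on a match and a xenophobic one otherwise.
; FillUp adds the supplied delta to the running fill level, with no clamping.
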(fn `BeingHeld`
  (params (handType :type String))
  (bind _asbp_customer (cast `/Game/CM_Game/Blueprints/BP_Customer` (`self.GetInstigator`)))
  (if (`KismetStringLibrary.EqualEqual_StrStr` handType (`/Game/CM_Game/Blueprints/BP_Customer.customerType` _asbp_customer))
    (`/Game/CM_Game/Blueprints/BP_Customer.Reaction` _asbp_customer 0)
    (else
      (`/Game/CM_Game/Blueprints/BP_Customer.Reaction` _asbp_customer 2) ; xenophobic reaction
    )))

(fn `FillUp`
  (params (level_dt :type "Float (double-precision)"))
  (set `self.fill_level` (+ level_dt (`self.fill_level`))))

(fn `UserConstructionScript`)