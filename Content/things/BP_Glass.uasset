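; A drink glass belonging to its instigator BP_Customer, whose name it displays, that tracks progress through a recipe of tagged ingredients.
; An overlapping actor tagged with the next task is destroyed and the task removed after its delay, through a gate that any end overlap closes.
; BeingHeld and DrinkComplete trigger customer reactions based on hand type and remaining tasks.
; FillUp accumulates and displays a fill level, separate from recipe completion.
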(event `self.ReceiveBeginPlay`
  (`TextRenderComponent.K2_SetText` (`self.TextRender`) (`KismetTextLibrary.Conv_StringToText` (`KismetSystemLibrary.GetDisplayName` (`self.GetInstigator`)))))

(event `self.Capsule.OnComponentBeginOverlap`
  (params (OverlappedComponent :type "PrimitiveComponent Object Reference") (OtherActor :type "Actor Object Reference") (OtherComp :type "PrimitiveComponent Object Reference") (OtherBodyIndex :type Integer) (bFromSweep :type Boolean) (SweepResult :type "HitResult Structure (by ref)"))
  (bind _recipe (`self.recipe`))
  (bind _tasks (`/Game/things/BP_Recipe.tasks` _recipe))
  (bind _task_times (`/Game/things/BP_Recipe.task_times` _recipe))
  (bind _returnvalue (`KismetArrayLibrary.Array_Length` _tasks))
  ;[1 1 1] Check if actor is tagged with expected ingredient
  (`KismetSystemLibrary.PrintString` (`KismetStringLibrary.Conv_IntToString` _returnvalue))
  (if (> _returnvalue 0)
    (if (`self.ActorHasTag` OtherActor (`|GetArrayItem` _tasks))
      (`KismetSystemLibrary.Delay` (`|GetArrayItem` _task_times))
      (`/Engine/EditorBlueprintResources/StandardMacros.Gate` false :!label _label
        (:`Exit`
          (`self.K2_DestroyActor` OtherActor)
          (`KismetArrayLibrary.Array_Remove` _tasks)
          (`KismetArrayLibrary.Array_Remove` _task_times)
          (goto _label :!via `Open`))))))

(event `self.Capsule.OnComponentEndOverlap`
  (params (OverlappedComponent :type "PrimitiveComponent Object Reference") (OtherActor :type "Actor Object Reference") (OtherComp :type "PrimitiveComponent Object Reference") (OtherBodyIndex :type Integer))
  ;[1 1 1] Check if actor is tagged with expected ingredient
  (if (== OtherActor (stale `self.Capsule.OnComponentBeginOverlap` OtherActor))
    (goto _label :!via `Close`)))

(fn `BeingHeld`
  (params (handType :type String))
  (bind _asbp_customer (cast `/Game/things/BP_Customer` (`self.GetInstigator`)))
  (if (`KismetStringLibrary.EqualEqual_StrStr` handType (`/Game/things/BP_Customer.customerType` _asbp_customer))
    (`/Game/things/BP_Customer.Reaction` _asbp_customer 0)
    (else
      (`/Game/things/BP_Customer.Reaction` _asbp_customer 2) ; xenophobic reaction
    )))

(fn `DrinkComplete`
  (bind _asbp_customer (cast `/Game/things/BP_Customer` (`self.GetInstigator`)))
  (if (== 0 (`KismetArrayLibrary.Array_Length` (`/Game/things/BP_Recipe.tasks` (`self.recipe`))))
    (`/Game/things/BP_Customer.Reaction` _asbp_customer 4)
    (else
      (`/Game/things/BP_Customer.Reaction` _asbp_customer 3) ; xenophobic reaction
    )))

(fn `FillUp`
  (params (level_dt :type "Float (double-precision)"))
  (set `self.fill_level` (+ level_dt (`self.fill_level`)))
  (`TextRenderComponent.K2_SetText` (`self.TextRender1`) (`KismetTextLibrary.Conv_DoubleToText` (`self.fill_level`) "HalfToEven")))

(fn `UserConstructionScript`)