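; BP_Nozzle is a pouring spout that emits falling fluid when tilted past TippingPoint and fills BP_Glass actors the fluid hits.
; Each tick it toggles the particles by tilt angle and sets their initial velocity from its own frame-to-frame movement, in local space, plus an upward offset.
; Particle collisions trigger a short line trace, and hits on a glass's capsule component call FillUp, scaled by FillSpeed and delta time.
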(event OnParticleCollide(falling_fluid)
  (params (EventName :type Name :default "None") (EmitterTime :type Float%20%28single-precision%29) (ParticleTime :type Integer) (Location :type Vector :default "0, 0, 0") (Velocity :type Vector :default "0, 0, 0") (Direction :type Vector :default "0, 0, 0") (Normal :type Vector :default "0, 0, 0") (BoneName :type Name :default "None") (PhysMat :type Physical%20Material%20Object%20Reference))
  (bind _outhit (Collision|LineTraceByChannel Location (+ Location Direction) "TraceTypeQuery1" false 0 "None"))
  (if (== (Utilities|GetClass (.hitcomponent _outhit)) "/Script/Engine.CapsuleComponent")
    (if (== (Utilities|GetClass (.hitactor _outhit)) "/Game/things/BP_Glass.BP_Glass_C")
      (bind _asbp_glass (Utilities|Casting|CastToBP_Glass (.hitactor _outhit)))
      (Default|FillUp _asbp_glass (* (Variables|Default|Getfill_speed) (Utilities|Time|GetWorldDeltaSeconds))))))

(event EventTick
  (params (DeltaSeconds :type Float%20%28single-precision%29))
  (bind _returnvalue (Transformation|GetActorLocation))
  (bind _falling_fluid (Variables|Default|Getfalling_fluid))
  (Components|Activation|SetActive _falling_fluid (> (Class|KismetMathLibrary|DegAcos (Math|Vector|DotProduct "0,0.000000,1.000000" (Transformation|GetActorUpVector self))) (Variables|Default|Gettipping_point)) false)
  ;[1 1 1] approximate and add velocity to particles
  (Effects|Components|ParticleSystem|SetVectorParameter _falling_fluid "init_vel" (+ (Math|Transform|InverseTransformDirection (Transformation|GetActorTransform) (|((x1-x0)/dt) _returnvalue (Variables|Default|GetoldLocation) (Utilities|Time|GetWorldDeltaSeconds))) "0, 0,50.000000"))
  (Variables|Default|SetoldLocation _returnvalue))

(fn ConstructionScript)